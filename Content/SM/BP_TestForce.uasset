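; BP_TestForce is a physics test actor that applies a one-time rightward force to its static mesh on BeginPlay.
; Tick throttles sampling with an accumulated delay, printing the mesh's mass, component velocity, physics linear velocity and the actor's velocity.
; A Launch flag set after the first sample lets it quit the game once actor velocity is near zero.
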(event `self.ReceiveBeginPlay`
  (`PrimitiveComponent.AddForce` (`self.StaticMeshComponent`) (* (`KismetMathLibrary.Vector_Right`) 200000.0) "None" false))

(event `self.ReceiveTick`
  (params (DeltaSeconds :type "Float (single-precision)"))
  (set `self.delay` (+ DeltaSeconds (`self.delay`)))
  (if (> (`self.delay`) (/ 1.0 100.0))
    (set `self.delay` 0.0)
    (`|ExecutionSequence`
      (:`then_0`
        (`KismetSystemLibrary.PrintString` (`KismetStringLibrary.Conv_DoubleToString` (`PrimitiveComponent.GetMass` (`self.StaticMeshComponent`)))))
      (:`then_1`
        (`KismetSystemLibrary.PrintString` (`KismetStringLibrary.Conv_VectorToString` (`SceneComponent.GetComponentVelocity` (`self.StaticMeshComponent`)))))
      (:`then_2`
        (bind _returnvalue (`PrimitiveComponent.GetPhysicsLinearVelocity` (`self.StaticMeshComponent`) "None"))
        (`KismetSystemLibrary.PrintString` (`KismetStringLibrary.Conv_VectorToString` _returnvalue)))
      (:`then_3`
        (`KismetSystemLibrary.PrintString` (`KismetStringLibrary.Conv_VectorToString` (`self.GetVelocity`))))
      (:`then_4`
        (if (== (`self.GetVelocity`) (0.0 0.0 0.0))
          (if (`self.launch`)
            (`KismetSystemLibrary.QuitGame` null "Quit"))))
      (:`then_5`
        (set `self.launch` true)))))

(fn `UserConstructionScript`)