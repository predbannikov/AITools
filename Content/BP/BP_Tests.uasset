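; BP_Tests is a debug test actor that compares the facing of two static mesh components.
; Every Tick it prints the forward vectors of StaticMesh and StaticMesh1, plus the difference between them, with zero duration so the on-screen readout stays live.
; The first value uses PrintText and the other two use PrintString; the construction script is empty.
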(event `self.ReceiveTick`
  (params (DeltaSeconds :type "Float (single-precision)"))
  (bind _returnvalue (`SceneComponent.GetForwardVector` (`self.StaticMesh1`)))
  (bind _returnvalue_2 (`SceneComponent.GetForwardVector` (`self.StaticMesh`)))
  (`KismetSystemLibrary.PrintText` (`KismetTextLibrary.Conv_VectorToText` _returnvalue_2) true true (struct :`G` 0.66 :`B` 1.0 :`A` 1.0) 0.0)
  (`KismetSystemLibrary.PrintString` (`KismetStringLibrary.Conv_VectorToString` _returnvalue) true true (struct :`G` 0.66 :`B` 1.0 :`A` 1.0) 0.0)
  (`KismetSystemLibrary.PrintString` (`KismetStringLibrary.Conv_VectorToString` (- _returnvalue_2 _returnvalue)) true true (struct :`G` 0.66 :`B` 1.0 :`A` 1.0) 0.0))

(fn `UserConstructionScript`)