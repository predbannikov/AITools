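; BP_Leg is a leg actor for keyboard-driven physics force testing.
; While a gate toggled by F is open, Tick applies force to Leg2 along the axis between two scene point components.
; R flips the direction, while J and K lower or raise the magnitude and print it.
; PrintArrowForce recomputes the force vector every Tick and draws it as a debug arrow.
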(event `Key|R`
  (params (Key :type "Key Structure"))
  (:`Pressed`
    (`/Engine/EditorBlueprintResources/StandardMacros.FlipFlop`
      (:`A`
        (set `self.direct` false))
      (:`B`
        (set `self.direct` true)))))

(event `Key|J`
  (params (Key :type "Key Structure"))
  (:`Pressed`
    (bind _output_get (set `self.force` (- (`self.force`) (`self.step`))))
    (`KismetSystemLibrary.PrintString` (`KismetStringLibrary.Conv_DoubleToString` _output_get) true true (struct :`G` 0.66 :`B` 1.0 :`A` 1.0) 1.0)))

(event `Key|K`
  (params (Key :type "Key Structure"))
  (:`Pressed`
    (bind _output_get (set `self.force` (+ (`self.step`) (`self.force`))))
    (`KismetSystemLibrary.PrintString` (`KismetStringLibrary.Conv_DoubleToString` _output_get) true true (struct :`G` 0.66 :`B` 1.0 :`A` 1.0) 1.0)))

(event `self.ReceiveTick`
  (params (DeltaSeconds :type "Float (single-precision)"))
  (`|ExecutionSequence`
    (:`then_0`
      (`/Engine/EditorBlueprintResources/StandardMacros.Gate` true :!label _label
        (:`Exit`
          (`PrimitiveComponent.AddForce` (`self.Leg2`) (* (`self.ForceForwardVector`) (`self.force`)) "None" false))))
    (:`then_1`
      (`self.printArrowForce`))))

(event `Key|F`
  (params (Key :type "Key Structure"))
  (:`Pressed`
    (`KismetSystemLibrary.PrintString` "f" true true (struct :`G` 0.66 :`B` 1.0 :`A` 1.0) 5.0)
    (goto _label :!via `Toggle`)))

(event `self.ReceiveBeginPlay`
  ;[1 0.1354 0.1354] Init
  (bind _output_get (set `self.controller` (`GameplayStatics.GetPlayerController` 0)))
  (`self.EnableInput` _output_get)
  (set `self.ForceForwardVector` (`KismetMathLibrary.GetForwardVector` (`KismetMathLibrary.FindLookAtRotation` (`SceneComponent.K2_GetComponentLocation` (`self.PointForForceStart`)) (`SceneComponent.K2_GetComponentLocation` (`self.PointForForceEnd`))))))

(fn `printArrowForce`
  (bind _returnvalue (`SceneComponent.K2_GetComponentLocation` (`self.PointForForceEnd`)))
  (bind _returnvalue_2 (`SceneComponent.K2_GetComponentLocation` (`self.PointForForceStart`)))
  (if (`self.direct`)
    (bind _output_get (set `self.ForceForwardVector` (`KismetMathLibrary.GetForwardVector` (`KismetMathLibrary.FindLookAtRotation` (`SceneComponent.K2_GetComponentLocation` (`self.PointForForceStart`)) (`SceneComponent.K2_GetComponentLocation` (`self.PointForForceEnd`))))))
    (`KismetSystemLibrary.DrawDebugArrow` _returnvalue_2 (+ (* _output_get 30.0) _returnvalue_2) 3.0 (struct :`R` 0.134436 :`B` 1.0 :`A` 1.0) 0.0 1.0)
    (else
      (bind _output_get_2 (set `self.ForceForwardVector` (`KismetMathLibrary.GetForwardVector` (`KismetMathLibrary.FindLookAtRotation` (`SceneComponent.K2_GetComponentLocation` (`self.PointForForceEnd`)) (`SceneComponent.K2_GetComponentLocation` (`self.PointForForceStart`))))))
      (`KismetSystemLibrary.DrawDebugArrow` _returnvalue (+ (* _output_get_2 30.0) _returnvalue) 3.0 (struct :`R` 0.134436 :`B` 1.0 :`A` 1.0) 0.0 1.0))))

(fn `UserConstructionScript`)